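; Game instance for MBA that offers helpers to set and fetch the first player's lobby and session info.
; The setters write a name to the LobbyPlayerState of player controller 0 and store a PlayerLobby struct built from it in PlayerInfo.
; The getters return that player state rather than the stored struct.
; The Session functions duplicate the Lobby ones, also working on LobbyPlayerState.
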(fn `GetPlayerLobbyInfo`
  (returns (LobbyPlayerState :type "/Game/MBA/Blueprints/PlayerState/LobbyPlayerState Object Reference"))
  (bind _aslobby_player_state (cast `/Game/MBA/Blueprints/PlayerState/LobbyPlayerState` (`Controller.PlayerState` (`GameplayStatics.GetPlayerController` 0))))
  (return _aslobby_player_state))

(fn `GetPlayerSessionInfo`
  (returns (LobbyPlayerState :type "/Game/MBA/Blueprints/PlayerState/LobbyPlayerState Object Reference"))
  (bind _aslobby_player_state (cast `/Game/MBA/Blueprints/PlayerState/LobbyPlayerState` (`Controller.PlayerState` (`GameplayStatics.GetPlayerController` 0))))
  (return _aslobby_player_state))

(fn `SetPlayerLobbyInfo`
  (params (Name :type Text))
  (bind _aslobby_player_state (cast `/Game/MBA/Blueprints/PlayerState/LobbyPlayerState` (`Controller.PlayerState` (`GameplayStatics.GetPlayerController` 0))))
  (bind _output_get (set `/Game/MBA/Blueprints/PlayerState/LobbyPlayerState.PlayerName` Name _aslobby_player_state))
  (set `self.PlayerInfo` (make `/Game/MBA/Blueprints/Struct/PlayerLobby` _output_get)))

(fn `SetPlayerSessionInfo`
  (params (Name :type Text))
  (bind _aslobby_player_state (cast `/Game/MBA/Blueprints/PlayerState/LobbyPlayerState` (`Controller.PlayerState` (`GameplayStatics.GetPlayerController` 0))))
  (bind _output_get (set `/Game/MBA/Blueprints/PlayerState/LobbyPlayerState.PlayerName` Name _aslobby_player_state))
  (set `self.PlayerInfo` (make `/Game/MBA/Blueprints/Struct/PlayerLobby` _output_get)))