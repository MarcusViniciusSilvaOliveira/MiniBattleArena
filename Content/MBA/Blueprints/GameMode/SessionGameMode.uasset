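; Game mode for a multiplayer session map that moves the game to Map_Game_1 once at least two players are present.
; On each PostLogin with authority, it checks the player count, waits briefly, then refills AllPlayersSession with the level's SessionPawn actors.
; It then issues a servertravel console command through player controller 0.
; A disconnected OpenLevel listen-server node is left unused.
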(event `self.K2_PostLogin`
  (params (NewPlayer :type "PlayerController Object Reference"))
  (`/Engine/EditorBlueprintResources/ActorMacros.Switch Has Authority`
    (:`Authority`
      (bind _returnvalue (`self.GetNumPlayers`))
      (if (>= _returnvalue 2)
        (`KismetArrayLibrary.Array_Clear` (`self.AllPlayersSession`))
        (`KismetSystemLibrary.Delay` 1.0)
        (bind _outactors (`GameplayStatics.GetAllActorsOfClass` "/Game/MBA/Blueprints/Pawns/SessionPawn.SessionPawn_C"))
        (set `self.AllPlayersSession` _outactors)
        (`KismetSystemLibrary.ExecuteConsoleCommand` "servertravel Map_Game_1" (`GameplayStatics.GetPlayerController` 0))))))

(fn `UserConstructionScript`)